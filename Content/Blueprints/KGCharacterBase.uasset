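; KGCharacterBase is a base character with a sword, montage-driven melee attacks, health and death.
; On BeginPlay it spawns a BaseSword and attaches it to the mesh's Sword socket.
; TryMelee plays the knight attack montage or, if already playing, can queue Attack2 through section chaining; TryMagic is an empty stub.
; AnyDamage reduces Health, then at zero runs a one-time death: movement stops, the death montage plays, and weapon and character are destroyed.
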(event `CreateSword`
  (bind _returnvalue (`|SpawnActorFromClass` "/Game/Blueprints/BaseSword.BaseSword_C" (`self.GetTransform`) "Undefined" "OverrideRootScale"))
  (`self.K2_AttachToComponent` _returnvalue (`self.Mesh`) "Sword" "SnapToTarget" "SnapToTarget" "SnapToTarget" false)
  (set `self.Weapon` _returnvalue))

(event `self.ReceiveBeginPlay`
  (`self.CreateSword`))

(event `TryMelee`
  (bind _returnvalue (`SkeletalMeshComponent.GetAnimInstance` (`self.Mesh`)))
  (bind _returnvalue_2 (`AnimInstance.Montage_GetCurrentSection` _returnvalue "/Game/Assets/Knight/Montage_KnightAttack.Montage_KnightAttack"))
  (if (`AnimInstance.Montage_IsActive` _returnvalue "/Game/Assets/Knight/Montage_KnightAttack.Montage_KnightAttack")
    (switch `name` _returnvalue_2
      (:`Attack1`
        (`AnimInstance.Montage_SetNextSection` _returnvalue _returnvalue_2 "Attack2" null)))
    (else
      (`self.PlayAnimMontage` "/Game/Assets/Knight/Montage_KnightAttack.Montage_KnightAttack" 1.0 "Attack1"))))

(event `TryMagic`)

(event `self.ReceiveAnyDamage`
  (params (Damage :type "Float (single-precision)") (DamageType :type "DamageType Object Reference") (InstigatedBy :type "Controller Object Reference") (DamageCauser :type "Actor Object Reference"))
  (bind _output_get (set `self.Health` (- (`self.Health`) Damage)))
  (if (<= _output_get 0.0)
    (`/Engine/EditorBlueprintResources/StandardMacros.DoOnce` false
      (:`Completed`
        (`CharacterMovementComponent.DisableMovement` (`self.CharacterMovement`))
        (bind _returnvalue (`self.PlayAnimMontage` "/Game/Assets/Knight/Montage_PlayerDeath.Montage_PlayerDeath"))
        (`KismetSystemLibrary.Delay` _returnvalue)
        (`self.K2_DestroyActor` (`self.Weapon`))
        (`self.K2_DestroyActor`)))))

(fn `UserConstructionScript`)